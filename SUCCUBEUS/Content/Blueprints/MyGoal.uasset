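; MyGoal is a goal actor that loses health when enemies reach it and triggers game over when that health runs out.
; An overlapping EnemyCubeAxe is destroyed and decrements GoalHealth by one.
; Tick polls GoalHealth and, on every frame it is zero or below, adds a new GameOver widget to the viewport and calls the player controller's ignore-move and ignore-look setters with false.
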(event `self.ReceiveActorBeginOverlap`
  (params (OtherActor :type "Actor Object Reference"))
  (bind _asenemycubeaxe_c (cast `/Game/Cubes/EnemyCubeAxe` OtherActor))
  (`self.K2_DestroyActor` _asenemycubeaxe_c)
  (set `self.goalHealth` (- (`self.goalHealth`) 1)))

(event `self.ReceiveTick`
  (params (DeltaSeconds :type "Float (single-precision)"))
  (bind _returnvalue (`GameplayStatics.GetPlayerController` 0))
  (if (<= (`self.goalHealth`) 0)
    (bind _returnvalue_2 (`|CreateWidget` "/Game/Blueprints/GameOver.GameOver_C"))
    (`UserWidget.AddToViewport` _returnvalue_2)
    (`PlayerController.SetIgnoreMoveInput` _returnvalue false)
    (`PlayerController.SetIgnoreLookInput` _returnvalue false)))

(fn `UserConstructionScript`)